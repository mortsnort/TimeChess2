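; Grid actor that lays out the floor tiles, labels each with its index and places the first unit on a hardcoded temporary start tile.
; The construction script builds a GridX by GridY instanced mesh that blocks a custom trace channel, caching tile transforms in TileTransform.
; BeginPlay spawns the number actors and unit from that array.
; Helpers convert tile-relative locations to world space and find a tile index by XY bounds.
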(event EventBeginPlay
  (bind _defaultsceneroot (Variables|Default|GetDefaultSceneRoot))
  (bind _returnvalue (Transformation|GetWorldTransform _defaultsceneroot))
  (for (_array_element _array_index) (Variables|Default|GetTileTransform)
    (bind _returnvalue_2 (Game|SpawnActorfromClass "/Game/Blueprints/ArrayNumber.ArrayNumber_C" (Math|Transform|MakeTransform (Math|Vector|MakeVector (+ (.x (.location _returnvalue)) (.x (.location _array_element)) 5e+01) (+ (.y (.location _returnvalue)) (.y (.location _array_element)) 5e+01) (+ (.z (.location _array_element)) 2e+01)) (.rotation _array_element) (.scale _array_element)) "Undefined" 0 0))
    (Rendering|Components|TextRender|SetText (Variables|/Game/Blueprints/ArrayNumber.ArrayNumber_C|GetTextRender _returnvalue_2) (Utilities|Text|ToText(Integer) _array_index)))
  (CallFunction|SpawnUnit 224))

(event Collision|EventActorBeginOverlap
  (params (OtherActor :type Actor%20Object%20Reference)))

(event EventTick
  (params (DeltaSeconds :type Float%20%28single-precision%29)))

(fn ConstructionScript
  (bind _grid_y (Variables|Default|GetGrid%20Y))
  (bind _returnvalue (AddComponent|AddInstancedStaticMeshComponent false (Math|Conversions|ToTransform(Vector) (Math|Vector|MakeVector 0.0 0.0 0.0))))
  (Collision|SetCollisionResponsetoChannel _returnvalue "ECC_GameTraceChannel1" "ECR_Block")
  (Components|StaticMesh|SetStaticMesh _returnvalue "/Game/StarterContent/Architecture/Small_floor.Small_floor")
  (bind _output_get (Variables|Default|SetInstanced%20Static%20Static%20Component%20Reference _returnvalue))
  (for _index (range 0 (- (* (Variables|Default|GetGrid%20X) (Variables|Default|GetGrid%20Y)) 1))
    (Components|InstancedStaticMesh|AddInstance _output_get (Math|Conversions|ToTransform(Vector) (Math|Vector|MakeVector (Math|Conversions|ToFloat(Integer) (* (/ _index _grid_y) 101)) (Math|Conversions|ToFloat(Integer) (* (Math|Integer|%(Integer) _index _grid_y) 101)) 0.0)))
    (Utilities|Array|Add (Variables|Default|GetTileTransform) (Math|Conversions|ToTransform(Vector) (Math|Vector|MakeVector (Math|Conversions|ToFloat(Integer) (* (/ _index _grid_y) 101)) (Math|Conversions|ToFloat(Integer) (* (Math|Integer|%(Integer) _index _grid_y) 101)) 0.0)))))

(fn GetArrayNumofVec
  (params (Vector :type Vector))
  (bind (_x _y) (Math|Vector|BreakVector Vector))
  (bind (_array_element _array_index) (Utilities|Array|ForEachLoopwithBreak (Variables|Default|GetTileTransform) :!label _label)
    (:LoopBody
      (if (Math|Boolean|ANDBoolean (>= _x (.x (+ (Transformation|GetWorldLocation (Variables|Default|GetDefaultSceneRoot)) (.location _array_element)))) (<= _x (+ (.x (+ (Transformation|GetWorldLocation (Variables|Default|GetDefaultSceneRoot)) (.location _array_element))) 1e+02)) (<= _y (+ (.y (+ (Transformation|GetWorldLocation (Variables|Default|GetDefaultSceneRoot)) (.location _array_element))) 1e+02)) (>= _y (.y (+ (Transformation|GetWorldLocation (Variables|Default|GetDefaultSceneRoot)) (.location _array_element)))))
        (goto _label Break)))
    (:Completed
      (return _array_index))))

(fn GetRealWorldLoc
  (params (RelLoc :type Vector))
  (return (+ RelLoc (Transformation|GetWorldLocation (Variables|Default|GetDefaultSceneRoot)))))

(fn SpawnUnit
  (params (SpawnLoc :type Integer))
  (bind _worldloc (CallFunction|GetRealWorldLoc (.location (Utilities|Array|Get(acopy) (Variables|Default|GetTileTransform) SpawnLoc))))
  (bind _returnvalue (Game|SpawnActorfromClass "/Game/Blueprints/FirstUnit.FirstUnit_C" (Math|Transform|MakeTransform (Math|Vector|MakeVector (+ (.X (Math|Vector|BreakVector _worldloc)) 5e+01) (+ (.Y (Math|Vector|BreakVector _worldloc)) 5e+01) (+ (.Z (Math|Vector|BreakVector _worldloc)) 5e+01)) "0.000000,-90.000000,0.000000" "1,1,1") "Undefined" 0 10 15 0 0 0 0 0))
  (Variables|/Game/Blueprints/Unit.Unit_C|SetCurrentLoc _returnvalue SpawnLoc))