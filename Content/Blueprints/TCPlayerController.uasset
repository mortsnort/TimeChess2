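; Player controller for a grid-based game that handles click-to-select and click-to-move of units.
; Left clicks trace under the cursor, treating an exact FirstUnit class match as a unit and any other hit as ground.
; Selecting a unit with none active shows range decals through the level's SpawnGrid.
; A ground click clears them and deselects, moving the unit only if the tile is in range and recording its new location.
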(event Custom|NewUnitSelected
  (bind _spawngridref (Variables|Default|GetSpawnGridRef))
  (bind _tiles (Default|GetTilesinRange _spawngridref (Variables|Default|GetSelectedUnit)))
  (Default|DecalTilesinRange _spawngridref _tiles))

(event EventBeginPlay
  (bind _outactors (Actor|GetAllActorsOfClass "/Game/Blueprints/SpawnGrid.SpawnGrid_C"))
  (Variables|Default|SetSpawnGridRef (Utilities|Array|Get(acopy) _outactors)))

(event EventTick
  (params (DeltaSeconds :type Float%20%28single-precision%29))
  (Variables|Default|SetPreviousMouseXLocation (.LocationX (Game|Player|GetMousePosition))))

(event Input|MouseEvents|LeftMouseButton
  (params (Key :type Key%20Structure))
  (bind _returnvalue (Game|GetPlayerController 0))
  (bind _spawngridref (Variables|Default|GetSpawnGridRef))
  (bind _hitresult (Game|Player|GetHitResultUnderCursorbyChannel _returnvalue "TraceTypeQuery1" true))
  (:Pressed
    (if (.bblockinghit _hitresult)
      (bind _newparam (CallFunction|WhatWasHit (.hitactor _hitresult)))
      (if (Utilities|Enum|Equal(Enum) _newparam "NewEnumerator0")
        (bind _asunit (Utilities|Casting|CastToUnit (.hitactor _hitresult)))
        (Variables|Default|SetSelectedUnit _asunit)
        (if (not (Variables|Default|GetIsUnitSelected))
          (Variables|Default|SetIsUnitSelected true)
          (CallFunction|NewUnitSelected))
        (elif (Utilities|Enum|Equal(Enum) _newparam "NewEnumerator1")
          (if (Variables|Default|GetIsUnitSelected)
            (bind _arrayindex (Default|GetArrayNumofVec (Variables|Default|GetSpawnGridRef) (.location _hitresult)))
            (CallFunction|MoveUnit (Variables|Default|GetSelectedUnit) _arrayindex)
            (Default|RemoveMoveDecals _spawngridref (Variables|/Game/Blueprints/SpawnGrid.SpawnGrid_C|GetRangeDecals _spawngridref))
            (Variables|Default|SetIsUnitSelected false)))))))

(fn ConstructionScript)

(fn HoverAttempt)

(fn WhatWasHit
  (params (HitActor :type Actor%20Object%20Reference))
  (if (== (Utilities|GetClass HitActor) "/Game/Blueprints/FirstUnit.FirstUnit_C")
    (return "NewEnumerator0")
    (else
      (return "NewEnumerator1"))))

(fn MoveUnit
  (params (UnitToMove :type Unit%20Object%20Reference) (WheretoMove :type Integer))
  (bind _spawngridref (Variables|Default|GetSpawnGridRef))
  ;[1 1 1] Unit move command on event click
  (bind _tiles (Default|GetTilesinRange (Variables|Default|GetSpawnGridRef) UnitToMove))
  (if (Utilities|Array|ContainsItem _tiles WheretoMove)
    (bind _worldloc (Default|GetRealWorldLoc _spawngridref (.location (Utilities|Array|Get(acopy) (Variables|/Game/Blueprints/SpawnGrid.SpawnGrid_C|GetTileTransform _spawngridref) WheretoMove))))
    (Transformation|SetActorLocation UnitToMove (Math|Vector|MakeVector (+ (.X (Math|Vector|BreakVector _worldloc)) 5e+01) (+ (.Y (Math|Vector|BreakVector _worldloc)) 5e+01) (+ (.Z (Math|Vector|BreakVector _worldloc)) 5e+01)) false false)
    (Utilities|Map|Add (Variables|/Game/Blueprints/SpawnGrid.SpawnGrid_C|GetUnitLocations (Variables|Default|GetSpawnGridRef)) WheretoMove UnitToMove)
    (Variables|/Game/Blueprints/Unit.Unit_C|SetCurrentLoc UnitToMove WheretoMove)))