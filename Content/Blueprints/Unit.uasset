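; Unit is a Blueprint that runs an on-screen countdown timer.
; Tick feeds a one-second Delay, which throttles the countdown to roughly one step per second without a timer handle.
; Each step writes TimeLeft to the OnScreenTimer text, then decrements it, stopping once it reaches -1 so zero is the last value shown.
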(event EventBeginPlay)

(event Collision|EventActorBeginOverlap
  (params (OtherActor :type Actor%20Object%20Reference)))

(event EventTick
  (params (DeltaSeconds :type Float%20%28single-precision%29))
  (Utilities|FlowControl|Delay 1.0)
  (if (not (== (Variables|Default|GetTimeLeft) -1))
    (CallFunction|DrawTimer)
    (CallFunction|UpdateTime)))

(fn ConstructionScript)

(fn DrawTimer
  (Rendering|Components|TextRender|SetText (Variables|Default|GetOnScreenTimer) (Utilities|Text|ToText(Integer) (Variables|Default|GetTimeLeft))))

(fn UpdateTime
  (Variables|Default|SetTimeLeft (- (Variables|Default|GetTimeLeft) 1)))